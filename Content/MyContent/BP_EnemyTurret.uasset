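; Enemy turret that fires BP_EnemyBullet from its firing point on an endless delay loop from BeginPlay.
; IsScattershot selects single shots or a volley of half-scale bullets with random yaw spread.
; When LookAtPlayer is set, Tick rotates it along the player-to-turret look-at vector, with VerticalFiring scaling height.
; Sight-radius checks are unwired, so firing ignores player distance.
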(event `self.ReceiveBeginPlay`
  (if (`self.IsScattershot`)
    (`self.ScatterShot`)
    (else
      (`self.Shoot`))))

(event `self.ReceiveTick`
  (params (DeltaSeconds :type "Float (single-precision)"))
  (`self.FollowPlayer` 0.0))

(event `Shoot`
  ;[1 0.405 0.1729] Fire at Player
  (`|SpawnActorFromClass` "/Game/MyContent/BP_EnemyBullet.BP_EnemyBullet_C" (`SceneComponent.GetSocketTransform` (`self.SM_FiringPoint`) "None" "RTS_World") "Undefined" "MultiplyWithRoot" null null)
  (`KismetSystemLibrary.Delay` (`self.FiringRate`))
  (`self.Shoot`))

(event `ScatterShot`
  (bind _returnvalue (`SceneComponent.GetSocketTransform` (`self.SM_FiringPoint`) "None" "RTS_World"))
  ;[1 0.8459 0.1582] Scatter Shot
  (for _ (range 1 (+ (`self.MaxScatterShot`) 1))
    (`|SpawnActorFromClass` "/Game/MyContent/BP_EnemyBullet.BP_EnemyBullet_C" (`KismetMathLibrary.MakeTransform` (.location _returnvalue) (`KismetMathLibrary.MakeRotator` (.roll (.rotation _returnvalue)) (.pitch (.rotation _returnvalue)) (+ (.yaw (.rotation _returnvalue)) (`KismetMathLibrary.RandomFloatInRange` -15.0 15.0))) (0.5 0.5 0.5)) "Undefined" "MultiplyWithRoot" null null))
  (`KismetSystemLibrary.Delay` (`self.FiringRate`))
  (`self.ScatterShot`))

(event `FollowPlayer`
  (params (DeltaSeconds :type "Float (single-precision)"))
  (bind (_returnvalue_x _returnvalue_y _returnvalue_z) (`KismetMathLibrary.BreakVector` (`self.K2_GetActorLocation`)))
  (bind (_returnvalue_x_2 _returnvalue_y_2 _returnvalue_z_2) (`KismetMathLibrary.BreakVector` (`self.K2_GetActorLocation` (`GameplayStatics.GetPlayerPawn` 0))))
  ;[0.2941 1 0.2196] Follow Player
  (if (`self.LookAtPlayer`)
    (`self.K2_SetActorRotation` (`KismetMathLibrary.FindLookAtRotation` (`KismetMathLibrary.MakeVector` _returnvalue_x_2 _returnvalue_y_2 (* _returnvalue_z_2 (`self.VerticalFiring`))) (`KismetMathLibrary.MakeVector` _returnvalue_x _returnvalue_y (* _returnvalue_z (`self.VerticalFiring`)))))))

(fn `UserConstructionScript`)