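; BP_FallingPlatform is a platform that vanishes after the third-person character stands on it too long, then respawns.
; Begin and end overlap on its Collision component set an on-platform flag and reset the timer.
; Tick accumulates time while occupied; at the limit, it hides the mesh and disables its collision instead of destroying it.
; A Delay then restores both, with debug prints showing contact and elapsed time.
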(event `self.Collision.OnComponentBeginOverlap`
  (params (OverlappedComponent :type "PrimitiveComponent Object Reference") (OtherActor :type "Actor Object Reference") (OtherComp :type "PrimitiveComponent Object Reference") (OtherBodyIndex :type Integer) (bFromSweep :type Boolean) (SweepResult :type "HitResult Structure (by ref)"))
  ;[0.3336 1 0.7227] Set Time On Platform
  (cast `/Game/ThirdPerson/Blueprints/BP_ThirdPersonCharacter` OtherActor)
  (`KismetSystemLibrary.PrintString` "OnPlatform")
  (set `self.PlayerOnPlatform` true)
  (set `self.TimeOnPlatform` 0.0 :!label _label))

(event `self.Collision.OnComponentEndOverlap`
  (params (OverlappedComponent :type "PrimitiveComponent Object Reference") (OtherActor :type "Actor Object Reference") (OtherComp :type "PrimitiveComponent Object Reference") (OtherBodyIndex :type Integer))
  ;[0.3336 1 0.7227] Set Time On Platform
  (cast `/Game/ThirdPerson/Blueprints/BP_ThirdPersonCharacter` OtherActor)
  (set `self.PlayerOnPlatform` false)
  (goto _label))

(event `self.ReceiveTick`
  (params (DeltaSeconds :type "Float (single-precision)"))
  (bind _sm_platform (`self.SM_Platform`))
  ;[1 0.06741 0] 'Destroy' Platform
  (if (`self.PlayerOnPlatform`)
    (set `self.TimeOnPlatform` (+ DeltaSeconds (`self.TimeOnPlatform`)))
    (`KismetSystemLibrary.PrintString` (`KismetStringLibrary.Conv_DoubleToString` (`self.TimeOnPlatform`)))
    (if (>= (`self.TimeOnPlatform`) (`self.PlatformTimeLimit`))
      (`SceneComponent.SetVisibility` (`self.SM_Platform`) false false)
      (`PrimitiveComponent.SetCollisionEnabled` (`self.SM_Platform`) "NoCollision")
      (`KismetSystemLibrary.Delay` (`self.RespawnDelay`))
      (`SceneComponent.SetVisibility` _sm_platform true false)
      (`PrimitiveComponent.SetCollisionEnabled` _sm_platform "QueryAndPhysics"))))

(fn `UserConstructionScript`)