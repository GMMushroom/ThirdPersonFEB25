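; BP_Enemy is a simple Goomba-style enemy that chases the player and drops a coin when defeated.
; PawnSensing sets a chase flag, and Tick moves and rotates the enemy relative to the player until the distance reaches the sight radius.
; Any overlap with the third-person character launches that character and costs the enemy one health.
; At zero health it spawns BP_Coin at its transform and destroys itself.
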(event `self.ReceiveActorBeginOverlap`
  (params (OtherActor :type "Actor Object Reference"))
  ;[1 0.6722 0.4037] Goomba
  (bind _asbp_third_person_character (cast `/Game/ThirdPerson/Blueprints/BP_ThirdPersonCharacter` OtherActor))
  (`self.LaunchCharacter` _asbp_third_person_character (`self.LaunchDistance`) false false)
  (set `self.Health` (- (`self.Health`) 1))
  (if (<= (`self.Health`) 0)
    (`self.DropLoot`)
    (`self.K2_DestroyActor`)))

(event `FollowPlayer`
  (bind (_returnvalue_x _returnvalue_y) (`KismetMathLibrary.BreakVector` (`self.K2_GetActorLocation`)))
  (bind (_returnvalue_x_2 _returnvalue_y_2) (`KismetMathLibrary.BreakVector` (`self.K2_GetActorLocation` (`GameplayStatics.GetPlayerPawn` 0))))
  ;[0.2941 1 0.2196] Follow Player
  (`self.AddMovementInput` (`KismetMathLibrary.Normal` (- (`self.K2_GetActorLocation` (`GameplayStatics.GetPlayerPawn` 0)) (`self.K2_GetActorLocation`))))
  (`self.K2_SetActorRotation` (`KismetMathLibrary.FindLookAtRotation` (`KismetMathLibrary.MakeVector` _returnvalue_x_2 _returnvalue_y_2) (`KismetMathLibrary.MakeVector` _returnvalue_x _returnvalue_y))))

(event `self.ReceiveTick`
  (params (DeltaSeconds :type "Float (single-precision)"))
  ;[0.2578 0.9402 1] Start/Stop Following
  (if (`self.SeesPawn`)
    (`self.FollowPlayer`)
    (if (>= (`KismetMathLibrary.Vector_Distance` (`self.K2_GetActorLocation` (`GameplayStatics.GetPlayerPawn` 0)) (`self.K2_GetActorLocation`)) (stale `self.PawnSensing.OnSeePawn` _output_get))
      (set `self.SeesPawn` false))))

(event `self.PawnSensing.OnSeePawn`
  (params (Pawn :type "Pawn Object Reference"))
  ;[0.2578 0.9402 1] Start/Stop Following
  (set `self.SeesPawn` true)
  (bind _output_get (set `self.Sight Radius` (`PawnSensingComponent.SightRadius` (`self.PawnSensing`)))))

(event `DropLoot`
  ;[1 0.9082 0.1812] Drop Loot
  (`|SpawnActorFromClass` "/Game/MyContent/BP_Coin.BP_Coin_C" (`self.GetTransform`) "Undefined" "MultiplyWithRoot" null null))

(fn `UserConstructionScript`)