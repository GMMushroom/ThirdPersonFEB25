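; BP_NPC is a talkable NPC that shows lines from its Dialogue array in an on-screen WP_Dialogue widget.
; Each Talk event advances TalkIndex, creating the UI when needed and removing it after the last line.
; A Player-tagged overlap shows the NPC's Widget, which turns toward the camera every tick.
; Leaving mid-dialogue closes and resets it but sets the Widget visible rather than hiding it.
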(event `self.ReceiveActorBeginOverlap`
  (params (OtherActor :type "Actor Object Reference"))
  (if (`self.ActorHasTag` OtherActor "Player")
    (`SceneComponent.SetVisibility` (`self.Widget`) true false)))

(event `self.ReceiveActorEndOverlap`
  (params (OtherActor :type "Actor Object Reference"))
  (if (`self.ActorHasTag` OtherActor "Player")
    (`self.UI`
      (:`then`
        (`Widget.RemoveFromParent` (`self.UI`))
        (set `self.TalkIndex` -1)
        (set `self.UI` null)
        (`SceneComponent.SetVisibility` (`self.Widget`) true false))
      (:`else`))))

(event `self.ReceiveTick`
  (params (DeltaSeconds :type "Float (single-precision)"))
  (`SceneComponent.K2_SetWorldRotation` (`self.Widget`) (`KismetMathLibrary.FindLookAtRotation` (`SceneComponent.K2_GetComponentLocation` (`self.Widget`)) (`SceneComponent.K2_GetComponentLocation` (`Actor.RootComponent` (`GameplayStatics.GetPlayerCameraManager` 0)))) false false))

(event `/Game/MyContent/BPI_Dialogue.Talk`
  (`/Engine/EditorBlueprintResources/StandardMacros.IncrementInt` (`self.TalkIndex`)
    (:`  `
      (if (< (`self.TalkIndex`) (`KismetArrayLibrary.Array_Length` (`self.Dialogue`)))
        (`self.UI`
          (:`then`
            _)
          (:`else`
            (bind _returnvalue (`|CreateWidget` "/Game/MyContent/WP_Dialogue.WP_Dialogue_C" (`GameplayStatics.GetPlayerController` 0)))
            (bind _output_get (set `self.UI` _returnvalue))
            (`UserWidget.AddToViewport` _output_get 0)))
        (`TextBlock.SetText` (`/Game/MyContent/WP_Dialogue.DialogueText` (`self.UI`)) (`KismetTextLibrary.Conv_StringToText` (`|GetArrayItem` (`self.Dialogue`) (`self.TalkIndex`))))
        (else
          (`Widget.RemoveFromParent` (`self.UI`))
          (set `self.TalkIndex` -1)
          (set `self.UI` null))))))

(fn `UserConstructionScript`)